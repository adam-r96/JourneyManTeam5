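; Speed boost pad that temporarily boosts and launches the third-person character when it overlaps the collision.
; The overlap raises walk speed and the character's custom time dilation, launches it along its forward vector and plays pickup and wind sounds.
; After a fixed delay it restores hard-coded speed and dilation, then fades the wind.
; A CanBoost flag blocks retriggering and re-arms only if the wind audio is still valid.
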(event OnComponentBeginOverlap(Collision)
  (params (OverlappedComponent :type Primitive%20Component%20Object%20Reference) (OtherActor :type Actor%20Object%20Reference) (OtherComp :type Primitive%20Component%20Object%20Reference) (OtherBodyIndex :type Integer) (bFromSweep :type Boolean) (SweepResult :type Hit%20Result%20Structure%20%28by%20ref%29))
  (bind _asbp_third_person_character_ajr (Utilities|Casting|CastToBP_ThirdPersonCharacter_AJR OtherActor))
  (if (Variables|Default|GetCanBoost)
    (Variables|Default|SetCanBoost false)
    (Audio|PlaySound2D "/Game/GameFiles/Sounds/Objects/pickup_powerup_Cue_AJR.pickup_powerup_Cue_AJR" 1.0 1.0 0.0 0 0)
    (Variables|/Script/Engine.CharacterMovementComponent|SetMaxWalkSpeed (Variables|/Script/Engine.Character|GetCharacterMovement _asbp_third_person_character_ajr) 1.2e+03)
    (Variables|/Script/Engine.Actor|SetCustomTimeDilation _asbp_third_person_character_ajr 1.5)
    (Character|LaunchCharacter _asbp_third_person_character_ajr (* (Transformation|GetActorForwardVector _asbp_third_person_character_ajr) (Variables|Default|GetLaunchStrength)) true false)
    (bind _returnvalue (Audio|SpawnSound2D "/Game/GameFiles/Sounds/Ambience/ambient_wind.ambient_wind" 1.0 1.0 0.0 0))
    (Variables|Default|SetWindAudio _returnvalue)
    (Utilities|FlowControl|Delay 3.0)
    (Variables|/Script/Engine.CharacterMovementComponent|SetMaxWalkSpeed (Variables|/Script/Engine.Character|GetCharacterMovement _asbp_third_person_character_ajr) 5.5e+02)
    (Variables|/Script/Engine.Actor|SetCustomTimeDilation _asbp_third_person_character_ajr 1.0)
    (Utilities|IsValid (Variables|Default|GetWindAudio)
      (:Is%20Valid
        (Audio|Components|Audio|FadeOut (Variables|Default|GetWindAudio) 0.5 0.0 "Linear" :!class /Script/Engine.AudioComponent)
        (Variables|Default|SetCanBoost true)))))

(fn ConstructionScript)