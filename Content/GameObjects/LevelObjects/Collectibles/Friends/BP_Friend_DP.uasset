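; Collectible friend actor that the player picks up by pressing F while standing inside its collision box.
; Overlap with BP_ThirdPersonCharacter_AJR toggles collection and input on the actor.
; Collecting increments the count on the player's C_Collect_DP, shows it in a temporary widget, hides the mesh, then destroys the actor after a delay.
; The construction script applies the chosen mesh and derives the box's size and offset from its bounds.
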(event OnComponentBeginOverlap(Collision)
  (params (OverlappedComponent :type Primitive%20Component%20Object%20Reference) (OtherActor :type Actor%20Object%20Reference) (OtherComp :type Primitive%20Component%20Object%20Reference) (OtherBodyIndex :type Integer) (bFromSweep :type Boolean) (SweepResult :type Hit%20Result%20Structure%20%28by%20ref%29))
  (bind _asbp_third_person_character_ajr (Utilities|Casting|CastToBP_ThirdPersonCharacter_AJR OtherActor))
  (Variables|Default|SetPlayerREF _asbp_third_person_character_ajr)
  (Variables|Default|SetCanCollectFriend? true)
  (Input|EnableInput (Game|GetPlayerController 0)))

(event OnComponentEndOverlap(Collision)
  (params (OverlappedComponent :type Primitive%20Component%20Object%20Reference) (OtherActor :type Actor%20Object%20Reference) (OtherComp :type Primitive%20Component%20Object%20Reference) (OtherBodyIndex :type Integer))
  (bind _asbp_third_person_character_ajr (Utilities|Casting|CastToBP_ThirdPersonCharacter_AJR OtherActor))
  (Variables|Default|SetPlayerREF _asbp_third_person_character_ajr)
  (Variables|Default|SetCanCollectFriend? false)
  (Input|DisableInput (Game|GetPlayerController 0)))

(event Input|KeyboardEvents|F
  (params (Key :type Key%20Structure :default "None"))
  (:Pressed
    (if (Variables|Default|GetCanCollectFriend?)
      (bind _returnvalue (UserInterface|CreateWidget "/Game/GameObjects/LevelObjects/Collectibles/Friends/WBP_FriendsCollected_DP.WBP_FriendsCollected_DP_C" (Game|GetPlayerController 0)))
      (Variables|Default|SetWidgetREF _returnvalue)
      (bind _returnvalue_2 (Default|IncreaseFriendsCollected (Actor|GetComponentbyClass (Variables|Default|GetPlayerREF) "/Game/GameObjects/LevelObjects/Collectibles/C_Collect_DP.C_Collect_DP_C")))
      (Variables|/Game/GameObjects/LevelObjects/Collectibles/Friends/WBP_FriendsCollected_DP.WBP_FriendsCollected_DP_C|SetFriendsCollected _returnvalue _returnvalue_2)
      (UserInterface|Viewport|AddtoViewport (Variables|Default|GetWidgetREF) 0)
      (Development|SetHiddeninGame (Variables|Default|GetFriend%20Mesh) true false)
      (Collision|SetCollisionEnabled (Variables|Default|GetCollision) "NoCollision")
      (Utilities|FlowControl|Delay 3.0)
      (Widget|RemovefromParent (Variables|Default|GetWidgetREF))
      (Actor|DestroyActor)
      (Development|PrintString "Friend destroyed" true true "(R=1.000000,G=0.000000,B=0.016606,A=1.000000)"))))

(fn ConstructionScript
  (bind _mesh (Variables|Construction|GetMesh))
  (bind _collision (Variables|Default|GetCollision))
  (bind _returnvalue (StaticMesh|GetBounds _mesh))
  (Components|StaticMesh|SetStaticMesh (Variables|Default|GetFriend%20Mesh) _mesh)
  (Components|Box|SetBoxExtent _collision (* (.boxextent _returnvalue) (Variables|Construction|GetCollisionScale)) true)
  (Transformation|SetRelativeLocation _collision (.boxextent _returnvalue) false false))