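; Shadow the Hedgehog variant of a collectible friend level object, built as a child Blueprint on a parent that supplies the base behavior.
; On BeginPlay it loops Shadow's idle animation on the skeletal mesh.
; Its PlayDanceAnim override runs the parent logic, then hides the mesh and disables collision on both the mesh and collision component, so Shadow disappears when the dance is triggered.
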(event EventBeginPlay
  (|CallParentFunction)
  (Components|Animation|PlayAnimation (Variables|Default|GetSkeletalMesh) "/Game/GameFiles/Animations/NPCS/AS_Shadow_The_Heghog_Idle.AS_Shadow_The_Heghog_Idle" true))

(fn ConstructionScript
  (|CallParentFunction))

(fn PlayDanceAnim
  (|CallParentFunction)
  (Rendering|SetVisibility (Variables|Default|GetSkeletalMesh) false false)
  (Collision|SetCollisionEnabled (Variables|Default|GetCollision) "NoCollision"))