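; Launch cannon level object that captures the player on overlap and fires them at a landing zone.
; On overlap it disables input and movement, detaches the camera boom from player transforms, caches the camera lock pose and snaps the player to a cannon socket.
; After a timed delay, LaunchPlayer detaches them, flags cannon flight and launches along a suggested custom arc with overridden gravity.
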(event OnComponentBeginOverlap(Sphere)
  (params (OverlappedComponent :type Primitive%20Component%20Object%20Reference) (OtherActor :type Actor%20Object%20Reference) (OtherComp :type Primitive%20Component%20Object%20Reference) (OtherBodyIndex :type Integer) (bFromSweep :type Boolean) (SweepResult :type Hit%20Result%20Structure%20%28by%20ref%29))
  (bind _asbp_third_person_character_ajr (Utilities|Casting|CastToBP_ThirdPersonCharacter_AJR OtherActor))
  (Variables|Default|SetCachedPlayer _asbp_third_person_character_ajr)
  (Variables|Default|SetPlayerInside true)
  (Variables|/Script/Engine.SceneComponent|SetbAbsoluteRotation (Variables|/Game/GameObjects/ThirdPersonBlueprints/Blueprints/BP_ThirdPersonCharacter_AJR.BP_ThirdPersonCharacter_AJR_C|GetCameraBoom (Variables|Default|GetCachedPlayer)) true)
  (Variables|/Script/Engine.SceneComponent|SetbAbsoluteLocation (Variables|/Game/GameObjects/ThirdPersonBlueprints/Blueprints/BP_ThirdPersonCharacter_AJR.BP_ThirdPersonCharacter_AJR_C|GetCameraBoom (Variables|Default|GetCachedPlayer)) true)
  (Input|DisableInput _asbp_third_person_character_ajr (Game|GetPlayerController 0))
  (Pawn|Components|CharacterMovement|DisableMovement (Variables|/Script/Engine.Character|GetCharacterMovement (Variables|Default|GetCachedPlayer)))
  (Variables|/Game/GameObjects/ThirdPersonBlueprints/Blueprints/BP_ThirdPersonCharacter_AJR.BP_ThirdPersonCharacter_AJR_C|SetCameraLockLocation (Variables|Default|GetCachedPlayer) (Transformation|GetActorLocation (Variables|Default|GetCachedPlayer)))
  (Variables|/Game/GameObjects/ThirdPersonBlueprints/Blueprints/BP_ThirdPersonCharacter_AJR.BP_ThirdPersonCharacter_AJR_C|SetCameraLockRotation (Variables|Default|GetCachedPlayer) (Transformation|GetActorRotation (Variables|Default|GetCachedPlayer)))
  (Transformation|AttachComponentToComponent OtherActor (Variables|Default|Getstylized_cannon_fbx) "PlayerPos" "SnapToTarget" "SnapToTarget" "KeepRelative" true)
  (Collision|SetCollisionEnabled (Variables|/Script/Engine.Character|GetMesh (Variables|Default|GetCachedPlayer)) "NoCollision")
  (Utilities|Time|SetTimerbyFunctionName 0 "LaunchPlayer" (Variables|Default|GetLaunchDelay)))

(event Custom|LaunchPlayer
  (bind _cachedplayer (Variables|Default|GetCachedPlayer))
  (bind _cachedplayer_2 (Variables|Default|GetCachedPlayer))
  (bind _returnvalue (Transformation|GetActorLocation _cachedplayer))
  (Transformation|DetachFromActor (Variables|Default|GetCachedPlayer) "KeepWorld" "KeepWorld" "KeepWorld")
  (bind _outlaunchvelocity (Game|SuggestProjectileVelocityCustomArc _returnvalue (Transformation|GetActorLocation (Variables|Default|GetLandingZone)) -2.94e+03 0.6))
  (Variables|/Game/GameObjects/ThirdPersonBlueprints/Blueprints/BP_ThirdPersonCharacter_AJR.BP_ThirdPersonCharacter_AJR_C|SetIsInCannonFlight _cachedplayer_2 true)
  (Transformation|SetActorLocation _cachedplayer_2 _returnvalue false false)
  (Pawn|Components|CharacterMovement|SetMovementMode (Variables|/Script/Engine.Character|GetCharacterMovement _cachedplayer_2) "MOVE_Walking" 0)
  (Character|LaunchCharacter _cachedplayer_2 (* _outlaunchvelocity "1.000000,1.000000,1.000000") true true)
  (Variables|Default|SetPlayerInside false)
  (Collision|SetCollisionEnabled (Variables|/Script/Engine.Character|GetCapsuleComponent (Variables|Default|GetCachedPlayer)) "QueryAndPhysics"))

(fn ConstructionScript)