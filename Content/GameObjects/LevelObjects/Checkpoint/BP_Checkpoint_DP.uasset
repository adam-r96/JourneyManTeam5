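; BP_Checkpoint_DP is a level checkpoint actor that saves the player's location when BP_ThirdPersonCharacter_AJR overlaps its collision.
; Save loads the "Checkpoint" slot or creates a BP_SaveCheckpoint, then writes the character's current location as LastCheckpointLocation.
; A successful write swaps the plane to the activated material, prints a message and sets IsActivated, which blocks further saves from that instance.
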(event OnComponentBeginOverlap(Collision)
  (params (OverlappedComponent :type Primitive%20Component%20Object%20Reference) (OtherActor :type Actor%20Object%20Reference) (OtherComp :type Primitive%20Component%20Object%20Reference) (OtherBodyIndex :type Integer) (bFromSweep :type Boolean) (SweepResult :type Hit%20Result%20Structure%20%28by%20ref%29))
  (bind _asbp_third_person_character_ajr (Utilities|Casting|CastToBP_ThirdPersonCharacter_AJR OtherActor))
  (CallFunction|Save (Transformation|GetActorLocation _asbp_third_person_character_ajr)))

(event EventBeginPlay)

(event Collision|EventActorBeginOverlap
  (params (OtherActor :type Actor%20Object%20Reference)))

(event EventTick
  (params (DeltaSeconds :type Float%20%28single-precision%29)))

(fn ConstructionScript)

(fn Save
  (params (Player%20Location :type Vector))
  (if (not (Variables|Default|GetisActivated))
    (bind _returnvalue (SaveGame|DoesSaveGameExist "Checkpoint"))
    (if _returnvalue
      (bind _returnvalue_2 (SaveGame|LoadGamefromSlot "Checkpoint"))
      (bind _asbp_save_checkpoint (Utilities|Casting|CastToBP_SaveCheckpoint _returnvalue_2))
      (Variables|/Game/GameObjects/LevelObjects/Checkpoint/BP_SaveCheckpoint.BP_SaveCheckpoint_C|SetLast%20Checkpoint%20Location _asbp_save_checkpoint Player%20Location)
      (bind _returnvalue_3 (SaveGame|SaveGametoSlot _asbp_save_checkpoint "Checkpoint"))
      (if _returnvalue_3
        (Rendering|Material|SetMaterial (Variables|Default|GetPlane) 0 "/Game/GameObjects/LevelObjects/Checkpoint/Material/M_CheckpointActivated.M_CheckpointActivated")
        (Variables|Default|SetisActivated true)
        (Development|PrintString "Checkpoint Saved" true true "(R=0.000000,G=1.000000,B=0.000000,A=1.000000)"))
      (else
        (bind _returnvalue_4 (SaveGame|CreateSaveGameObject "/Game/GameObjects/LevelObjects/Checkpoint/BP_SaveCheckpoint.BP_SaveCheckpoint_C"))
        (Variables|/Game/GameObjects/LevelObjects/Checkpoint/BP_SaveCheckpoint.BP_SaveCheckpoint_C|SetLast%20Checkpoint%20Location _returnvalue_4 Player%20Location)
        (bind _returnvalue_5 (SaveGame|SaveGametoSlot _returnvalue_4 "Checkpoint"))
        (if _returnvalue_5
          (Rendering|Material|SetMaterial (Variables|Default|GetPlane) 0 "/Game/GameObjects/LevelObjects/Checkpoint/Material/M_CheckpointActivated.M_CheckpointActivated")
          (Variables|Default|SetisActivated true)
          (Development|PrintString "Checkpoint Saved" true true "(R=0.000000,G=1.000000,B=0.000000,A=1.000000)"))))))