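; BP_Breakable is a level object that shatters into physics gibs when any attack contacts it.
; On BeginPlay it pre-spawns one hidden BP_Gib per BreakableGibs entry, with physics and collision off, and stores the references.
; Destroy calls OnBreak, plays the break sound, then moves the gibs to the mesh's transform and reveals them.
; Each gib gets physics-only collision and a random impulse and spin before the breakable destroys itself.
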(event Custom|Destroy
  (Default|CallOnBreak)
  (Audio|PlaySoundatLocation (Variables|Breakable|Details|Getbreakable_sound) (Transformation|GetWorldLocation (Variables|Default|GetMesh)) "0, 0, 0" 1.0 1.0 0.0 0 0 0 0)
  (CallFunction|TriggerGibs)
  (Actor|DestroyActor))

(event EventBeginPlay
  (CallFunction|SpawnGibs))

(event Collision|EventActorBeginOverlap
  (params (OtherActor :type Actor%20Object%20Reference)))

(event EventTick
  (params (DeltaSeconds :type Float%20%28single-precision%29)))

(event EventAnyAttackContact
  (CallFunction|Destroy))

(fn ConstructionScript)

(fn SpawnGibs
  (for (_array_element _array_index) (Variables|Breakable|Details|Getbreakable_gibs)
    (bind _returnvalue (Game|SpawnActorfromClass "/Game/GameObjects/LevelObjects/Breakables/BP_Gib.BP_Gib_C" (Math|Transform|MakeTransform (Transformation|GetWorldLocation (Variables|Default|GetMesh)) "0, 0, 0" "1.000000,1.000000,1.000000") "AlwaysSpawn" "MultiplyWithRoot" 0 _array_element _array_index (Variables|Breakable|Details|Getgib_lifetime) 0))
    (Utilities|Array|Add (Variables|Default|GetgibsReferences) _returnvalue)
    (Rendering|SetActorHiddenInGame _returnvalue true)
    (Physics|SetSimulatePhysics (Variables|/Game/GameObjects/LevelObjects/Breakables/BP_Gib.BP_Gib_C|GetStaticMesh _returnvalue) false)
    (Collision|SetCollisionEnabled (Variables|/Game/GameObjects/LevelObjects/Breakables/BP_Gib.BP_Gib_C|GetStaticMesh _returnvalue) "NoCollision")))

(fn TriggerGibs
  (bind _mesh (Variables|Default|GetMesh))
  (for _array_element (Variables|Default|GetgibsReferences)
    (Rendering|SetActorHiddenInGame _array_element false)
    (Transformation|SetActorLocation _array_element (Transformation|GetWorldLocation _mesh) false false)
    (Transformation|SetActorRotation _array_element (Transformation|GetWorldRotation _mesh))
    (Default|GibsEnabled _array_element)
    (Physics|SetSimulatePhysics (Variables|/Game/GameObjects/LevelObjects/Breakables/BP_Gib.BP_Gib_C|GetStaticMesh _array_element) true)
    (Collision|SetCollisionEnabled (Variables|/Game/GameObjects/LevelObjects/Breakables/BP_Gib.BP_Gib_C|GetStaticMesh _array_element) "PhysicsOnly")
    (Physics|AddImpulse (Variables|/Game/GameObjects/LevelObjects/Breakables/BP_Gib.BP_Gib_C|GetStaticMesh _array_element) (* (Math|Random|RandomUnitVectorinConeinDegrees "0.000000,0.000000,1.000000" 1.8e+02) (Math|Random|RandomFloatinRange 7e+02 2e+03)) "None" true)
    (Class|PrimitiveComponent|SetPhysicsAngularVelocityinDegrees (Variables|/Game/GameObjects/LevelObjects/Breakables/BP_Gib.BP_Gib_C|GetStaticMesh _array_element) (* (Math|Random|RandomUnitVectorinConeinDegrees "0.000000,0.000000,1.000000" 3.6e+02) (Math|Random|RandomFloatinRange 3e+02 5e+02)) false "None")))