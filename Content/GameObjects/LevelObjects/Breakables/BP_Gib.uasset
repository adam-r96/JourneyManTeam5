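; BP_Gib is a breakable debris piece that shows an assigned gib mesh and removes itself after a lifetime.
; When gibs are enabled, a timer triggers Dissolve after LifeTime plus a small Index-based stagger.
; Dissolve turns off physics, collision and visibility, then activates Niagara if the mesh was recently rendered, destroying the actor when the effect finishes.
; Gibs not recently rendered skip the effect and are destroyed immediately.
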(event OnSystemFinished(Niagara)
  (params (PSystem :type Niagara%20Component%20Object%20Reference))
  (Actor|DestroyActor))

(event Custom|Dissolve
  (Physics|SetSimulatePhysics (Variables|Default|GetStaticMesh) false)
  (Collision|SetCollisionEnabled (Variables|Default|GetStaticMesh) "NoCollision")
  (Rendering|SetVisibility (Variables|Default|GetStaticMesh) false false)
  (if (Class|PrimitiveComponent|WasRecentlyRendered (Variables|Default|GetStaticMesh) 0.2)
    (Components|Activation|SetActive (Variables|Default|GetNiagara) true false)
    (else
      (Actor|DestroyActor))))

(event Custom|GibsEnabled
  (Utilities|Time|SetTimerbyEvent (delegate Custom|Dissolve) (+ (* (Math|Conversions|ToFloat(Integer) (+ (Variables|Default|GetIndex) 1)) 0.02) (Variables|Default|GetLifeTime))))

(fn ConstructionScript
  (Components|StaticMesh|SetStaticMesh (Variables|Default|GetStaticMesh) (Variables|Default|GetGibMesh)))