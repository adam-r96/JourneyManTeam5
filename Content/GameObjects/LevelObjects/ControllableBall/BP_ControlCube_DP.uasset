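; BP_ControlCube_DP is an interactable cube that lets the player toggle control of a ball, though so far it only freezes the character and prints debug text.
; Its trigger overlap stores the third-person character and shows an interact widget, which is removed on exit.
; While the player is on the cube, Interact flip-flops between disabling character movement and restoring walking; otherwise it prints that the player is off the cube.
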(event OnComponentBeginOverlap(Trigger)
  (params (OverlappedComponent :type Primitive%20Component%20Object%20Reference) (OtherActor :type Actor%20Object%20Reference) (OtherComp :type Primitive%20Component%20Object%20Reference) (OtherBodyIndex :type Integer) (bFromSweep :type Boolean) (SweepResult :type Hit%20Result%20Structure%20%28by%20ref%29))
  (bind _asbp_third_person_character_ajr (Utilities|Casting|CastToBP_ThirdPersonCharacter_AJR OtherActor))
  (bind _output_get (Variables|Default|SetCharacterREF _asbp_third_person_character_ajr))
  (bind _returnvalue (UserInterface|CreateWidget "/Game/GameObjects/LevelObjects/ControllableBall/WBP_CubeInteract_DP.WBP_CubeInteract_DP_C" (Pawn|GetLocalViewingPlayerController _output_get)))
  (bind _output_get_2 (Variables|Default|SetWidgetREF _returnvalue))
  (UserInterface|Viewport|AddtoViewport _output_get_2 0)
  (Variables|Default|SetIsOnCube? true))

(event OnComponentEndOverlap(Trigger)
  (params (OverlappedComponent :type Primitive%20Component%20Object%20Reference) (OtherActor :type Actor%20Object%20Reference) (OtherComp :type Primitive%20Component%20Object%20Reference) (OtherBodyIndex :type Integer))
  (bind _asbp_third_person_character_ajr (Utilities|Casting|CastToBP_ThirdPersonCharacter_AJR OtherActor))
  (Variables|Default|SetCharacterREF _asbp_third_person_character_ajr)
  (Widget|RemovefromParent (Variables|Default|GetWidgetREF))
  (Variables|Default|SetIsOnCube? false))

(event EventInteract
  (if (Variables|Default|GetIsOnCube?)
    (Utilities|FlowControl|FlipFlop
      (:A
        ;[0.15 0.15 0.15 0.5] Control Ball
        (Pawn|Components|CharacterMovement|DisableMovement (Variables|/Script/Engine.Character|GetCharacterMovement (Variables|Default|GetCharacterREF)))
        (Development|PrintString "In control of ball"))
      (:B
        ;[0.15 0.15 0.15 0.5] Stop Controlling Ball
        (Pawn|Components|CharacterMovement|SetMovementMode (Variables|/Script/Engine.Character|GetCharacterMovement (Variables|Default|GetCharacterREF)) "MOVE_Walking" 0)
        (Development|PrintString "In control of player")))
    (else
      (Development|PrintString "Player is not on control cube"))))

(fn ConstructionScript)