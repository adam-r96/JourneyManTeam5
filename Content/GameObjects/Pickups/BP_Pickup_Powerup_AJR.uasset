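; Powerup pickup that grants the player the powerup from its PickupPowerup data asset when collected.
; On BeginPlay it binds to the item picked up event, which passes that asset to the instigator through PlayerPowerupNew.
; The construction script blocking-loads the asset's mesh and applies a powerup overlay material.
; A missing asset or failed mesh load shows a dev error mesh instead.
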(event Custom|ItemPickedUp_Event
  (params (Instigator :type BP%20Third%20Person%20Character%20AJR%20Object%20Reference))
  ;[0.15 0.15 0.15 0.5] Give the player the powerup attached to this
  (bind _pickup_powerup (Variables|Pickup|Powerup|Getpickup_powerup)
    (:then
      (Default|PlayerPowerupNew Instigator _pickup_powerup))
    (:else)))

(event EventBeginPlay
  (EventDispatchers|BindEventtoItemPickedUp (delegate Custom|ItemPickedUp_Event)))

(fn ConstructionScript
  (|CallParentFunction)
  ;[0.15 0.15 0.15 0.5] Load the static mesh from the powerup data asset
  (bind _pickup_powerup (Variables|Pickup|Powerup|Getpickup_powerup)
    (:then
      (bind _returnvalue (Utilities|LoadAssetBlocking (Variables|/Game/GameObjects/Abilities/Powerups/PDA_Powerup_AJR.PDA_Powerup_AJR_C|GetPowerup%20Pickup%20Mesh _pickup_powerup)))
      (bind _asstatic_mesh (Utilities|Casting|CastToStaticMesh _returnvalue)
        (:then
          ;[0.15 0.15 0.15 0.5] Set the static mesh to the data asset
          (Components|StaticMesh|SetStaticMesh (Variables|Default|GetPickup%20%20Mesh) _asstatic_mesh)
          (Rendering|Material|SetOverlayMaterial (Variables|Default|GetPickup%20%20Mesh) "/Game/GameFiles/Materials/Overlays/MI_Overlay_Powerup_AJR.MI_Overlay_Powerup_AJR" :!class /Script/Engine.MeshComponent))
        (:CastFailed
          ;[0.15 0.15 0.15 0.5] If anything is invalid, the model will be an error text
          (Components|StaticMesh|SetStaticMesh (Variables|Default|GetPickup%20%20Mesh) "/Game/GameFiles/Models/Dev/Error/sm_dev_error.sm_dev_error" :!label _label))))
    (:else
      (goto _label))))