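; Base pickup actor that reacts when the third-person character overlaps its range, broadcasting ItemPickedUp and playing a particle and sound.
; It then disables range collision and runs one of two animation styles before destroying itself.
; Fade swaps in a dynamic material and lowers its opacity.
; Magnet chains two timelines, floating the pickup upward, then pulling it toward the player's bounds center while shrinking it.
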(event OnComponentBeginOverlap(PickupRange)
  (params (OverlappedComponent :type Primitive%20Component%20Object%20Reference) (OtherActor :type Actor%20Object%20Reference) (OtherComp :type Primitive%20Component%20Object%20Reference) (OtherBodyIndex :type Integer) (bFromSweep :type Boolean) (SweepResult :type Hit%20Result%20Structure%20%28by%20ref%29))
  (bind _asbp_third_person_character_ajr (Utilities|Casting|CastToBP_ThirdPersonCharacter_AJR OtherActor))
  (bind _output_get (Variables|Default|SetpickupPlayerRef _asbp_third_person_character_ajr))
  (Default|CallItemPickedUp _output_get)
  ;[0.15 0.15 0.15 0.5] Spawn a particle when picking up an object
  (Niagara|SpawnSystematLocation (Variables|Pickup|Details|Getpickup_details_particles) (Transformation|GetWorldLocation (Variables|Default|GetPickup%20%20Mesh)))
  ;[0.15 0.15 0.15 0.5] Play a sound
  (Audio|PlaySoundatLocation (Variables|Pickup|Details|Getpickup_details_sound) (Transformation|GetActorLocation) "0, 0, 0" 1.0 1.0 0.0 0 0 0 0)
  ;[0.15 0.15 0.15 0.5] Start the pickup anim
  (CallFunction|PickupAnimation))

(event Custom|pickup_animation
  (Collision|SetCollisionEnabled (Variables|Default|GetPickup%20Range) "NoCollision")
  (switch Utilities|FlowControl|Switch|Switchonenum_pickupAnimationStyle (Variables|Pickup|Animation|Getpickup_animation_style)
    (:NewEnumerator0
      (CallFunction|PickupMeshSetFadeMaterial)
      (CallFunction|PickupAnimFade))
    (:NewEnumerator1
      (CallFunction|PickupAnimMagnet))))

(event Custom|pickup_anim_fade
  (bind _alpha (Timeline|timeline_pickupAnim_fade PlayFromStart)
    (:Update
      (Rendering|Material|SetScalarParameterValue (Variables|Default|GetMID_PickupFade) "Opacity" (- 1.0 _alpha) :!class /Script/Engine.MaterialInstanceDynamic))
    (:Finished
      (Actor|DestroyActor))))

(event Custom|pickup_anim_magnet
  (CallFunction|PickupAnimMagnetCalculateVectors)
  (bind _alpha (Timeline|timeline_pickupAnim_magnet_up PlayFromStart)
    (:Update
      (Transformation|SetActorLocation (Math|Vector|Lerp(Vector) (Variables|Default|Getanim_magnet_start) (Variables|Default|Getanim_magnet_end) _alpha) false false))
    (:Finished
      (bind _alpha_2 (Timeline|timeline_pickupAnim_magnet_drag PlayFromStart)
        (:Update
          (Transformation|SetActorLocation (Math|Vector|Lerp(Vector) (Transformation|GetActorLocation) (.Origin (Collision|GetActorBounds (Variables|Default|GetpickupPlayerRef) true false)) _alpha_2) false false)
          (Transformation|SetActorScale3D (Math|Vector|MakeVector (- 1.0 _alpha_2) (- 1.0 _alpha_2) (- 1.0 _alpha_2))))
        (:Finished
          (Actor|DestroyActor))))))

(fn ConstructionScript
  ;[0.15 0.15 0.15 0.5] Set the float up animation time in seconds
  (Components|Timeline|SetPlayRate (Variables|Default|Gettimeline_pickupAnim_fade) (/ 1.0 (Variables|Pickup|Animation|Getpickup_animation_floatUp_time))))

(fn PickupMeshSetFadeMaterial
  (bind _returnvalue (Rendering|Material|CreateDynamicMaterialInstance "/Game/GameFiles/Materials/Special/M_PickupFade.M_PickupFade" "None" "None" :!class /Script/Engine.KismetMaterialLibrary))
  (Variables|Default|SetMID_PickupFade _returnvalue)
  (for _array_element (Rendering|Material|GetMaterials (Variables|Default|GetPickup%20%20Mesh))
    (Rendering|Material|SetMaterial (Variables|Default|GetPickup%20%20Mesh) 0 (Variables|Default|GetMID_PickupFade))))

(fn PickupAnimMagnetCalculateVectors
  (bind _output_get (Variables|Default|Setanim_magnet_start (Transformation|GetActorLocation)))
  (Variables|Default|Setanim_magnet_end (+ _output_get (Math|Vector|MakeVector 0.0 0.0 (Variables|Pickup|Animation|Getpickup_animation_magnet_floatUpDistance)))))