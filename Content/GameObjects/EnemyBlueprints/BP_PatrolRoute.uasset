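; BP_PatrolRoute is a spline-based patrol route that supplies world-space waypoints, apparently for enemy patrols.
; It stores the current point index and direction, and each PatrolPath call advances the index one step, reversing at either end for back-and-forth traversal.
; GetSplinePointWorldPos returns the current point's world location.
; The patrol state lives on the route itself, and the construction script is empty.
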(event Custom|PatrolPath
  (bind _output_get (Variables|Default|SetPatrolPoint (+ (Variables|Default|GetPatrolPoint) (Variables|Default|GetDirection))))
  (if (== _output_get (- (Spline|GetNumberOfSplinePoints (Variables|Default|GetPatrolRoute)) 1))
    (Variables|Default|SetDirection -1)
    (elif (== (Variables|Default|GetPatrolPoint) 0)
      (Variables|Default|SetDirection 1))))

(fn ConstructionScript)

(fn GetSplinePointWorldPos
  (return (Spline|GetLocationatSplinePoint (Variables|Default|GetPatrolRoute) (Variables|Default|GetPatrolPoint) "World")))