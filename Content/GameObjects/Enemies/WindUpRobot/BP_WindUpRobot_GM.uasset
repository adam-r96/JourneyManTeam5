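; Wind-up robot enemy that patrols points, chases the player and damages them through its front hitbox.
; Tick turns it at a clamped yaw speed before issuing AI MoveTo, so clunky turn-then-move motion leaves its key easier to hit.
; Sphere overlap switches patrol to attack, which re-aims when the player leaves its forward cone and reverts beyond aggro range.
; Spin attack contacts increment a counter that destroys it at a threshold.
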(event OnComponentBeginOverlap(Hitbox_Front)
  (params (OverlappedComponent :type Primitive%20Component%20Object%20Reference) (OtherActor :type Actor%20Object%20Reference) (OtherComp :type Primitive%20Component%20Object%20Reference) (OtherBodyIndex :type Integer) (bFromSweep :type Boolean) (SweepResult :type Hit%20Result%20Structure%20%28by%20ref%29))
  (bind _asbp_third_person_character_ajr (Utilities|Casting|CastToBP_ThirdPersonCharacter_AJR OtherActor))
  (Class|BPIDamagePlayer|DamagePlayer(Message) _asbp_third_person_character_ajr))

(event OnComponentBeginOverlap(DetectionSphere)
  (params (OverlappedComponent :type Primitive%20Component%20Object%20Reference) (OtherActor :type Actor%20Object%20Reference) (OtherComp :type Primitive%20Component%20Object%20Reference) (OtherBodyIndex :type Integer) (bFromSweep :type Boolean) (SweepResult :type Hit%20Result%20Structure%20%28by%20ref%29))
  ;[0.15 0.15 0.15 0.5] Change to attack state if Player is in range of enemy
  (bind _asbp_third_person_character_ajr (Utilities|Casting|CastToBP_ThirdPersonCharacter_AJR OtherActor))
  (Variables|Default|SetPlayerReference _asbp_third_person_character_ajr)
  (Variables|Default|SetCurrentState "NewEnumerator1")
  (CallFunction|StartAttack))

(event Custom|MoveToNextPatrolPoint
  ;[0.15 0.15 0.15 0.5] Calculate the rotation thats needed to face the next patrol point, and begin to rotate to it
  (Variables|Default|SetTargetRotation (Math|Rotator|FindLookatRotation (Transformation|GetActorLocation self) (Transformation|GetActorLocation (Utilities|Array|Get(acopy) (Variables|Default|GetPatrolPoints) (Variables|Default|GetPatrolIndex)))))
  (Variables|Default|SetIsRotating true))

(event Custom|StartAttack
  (bind _self self)
  ;[0.15 0.15 0.15 0.5] Stop moving along patrol, calculate the rotation needed to face the players current position, then hand control over to rotation system in event tick
  (Components|Movement|StopMovementImmediately (Variables|Character|GetCharacterMovement _self))
  (Variables|Default|SetIsCharging false)
  (Variables|Default|SetTargetRotation (Math|Rotator|FindLookatRotation (Transformation|GetActorLocation _self) (Transformation|GetActorLocation (Variables|Default|GetPlayerReference))))
  (Variables|Default|SetIsRotating true))

(event Custom|Movement
  ;[0.15 0.15 0.15 0.5] Either move between the different patrol points in patrol mode, or towards the player in attack mode
  (if (Utilities|Enum|Equal(Enum) (Variables|Default|GetCurrentState) "NewEnumerator0")
    (AI|AIMoveTo self "0, 0, 0" (Utilities|Array|Get(acopy) (Variables|Default|GetPatrolPoints) (Variables|Default|GetPatrolIndex)) 5.0 false
      (:OnSuccess
        (Variables|Default|SetPatrolIndex (Math|Integer|%(Integer) (+ (Variables|Default|GetPatrolIndex) 1) (Utilities|Array|Length (Variables|Default|GetPatrolPoints))))
        (CallFunction|MovetoNextPatrolPoint)))
    (else
      (AI|AIMoveTo self "0, 0, 0" (Variables|Default|GetPlayerReference) 5.0 false
        (:OnSuccess
          (Variables|Default|SetPatrolIndex (Math|Integer|%(Integer) (+ (Variables|Default|GetPatrolIndex) 1) (Utilities|Array|Length (Variables|Default|GetPatrolPoints))))
          (CallFunction|MovetoNextPatrolPoint))))))

(event EventSpinAttackContact
  (params (HitInfo :type Hit%20Result%20Structure))
  ;[0.15 0.15 0.15 0.5] When the player attacks the wind up key with a spin attack, add to the hit counter. After 3 hits, the enemy is destroyed.
  (bind _result (Math|Integer|IncrementInt (Variables|Default|GetHitCounter))
    (:%20%20
      (if (>= _result 18)
        (Actor|DestroyActor)))))

(event EventBeginPlay
  ;[0.15 0.15 0.15 0.5] On run, begin patrol sequence
  (CallFunction|MovetoNextPatrolPoint))

(event EventTick
  (params (DeltaSeconds :type Float%20%28single-precision%29))
  (bind _self self)
  (bind _returnvalue (Transformation|GetActorRotation _self))
  ;[0.15 0.15 0.15 0.5] Check whether the enemy is in Patrol or Attack state
  (if (Utilities|Enum|Equal(Enum) (Variables|Default|GetCurrentState) "NewEnumerator0")
    ;[0.15 0.15 0.15 0.5] on each frame, if the robot is rotating, interpolate (smoothly transition between two values over time, trying to simulate a clunky robot) its rotation towards the target point. Once the yaw is within 10 degrees, mark rotation as complete and issue the move command. On arrival, advance the patrol index and loop back. This event means the robot rotates and then moves, not doing both at once, making it easier for the player to attack its key hitbox.
    (if (Variables|Default|GetIsRotating) :!label _label
      (Transformation|SetActorRotation (Math|Rotator|MakeRotator 0.0 0.0 (+ (.yaw _returnvalue) (Math|Float|Clamp(Float) (Math|Rotator|NormalizeAxis (- (.yaw (Variables|Default|GetTargetRotation)) (.yaw _returnvalue))) (* (* (Variables|Default|GetRotationSpeed) DeltaSeconds) -1.0) (* (Variables|Default|GetRotationSpeed) DeltaSeconds)))))
      (if (< (Math|Float|Absolute(Float) (- (.yaw (Transformation|GetActorRotation self)) (.yaw (Variables|Default|GetTargetRotation)))) 1e+01)
        (Variables|Default|SetIsRotating false)
        (CallFunction|Movement)))
    (elif (Utilities|Enum|Equal(Enum) (Variables|Default|GetCurrentState) "NewEnumerator1")
      (if (> (Transformation|GetDistanceTo self (Variables|Default|GetPlayerReference)) (Variables|Default|GetAggroRange))
        ;[0.15 0.15 0.15 0.5] If the player leaves aggro-range, return to patrol.
        (Variables|Default|SetCurrentState "NewEnumerator0")
        (Variables|Default|SetIsRotating false)
        (Variables|Default|SetIsCharging false)
        (CallFunction|MovetoNextPatrolPoint)
        (elif (Variables|Default|GetIsRotating)
          (goto _label)
          (elif (< (Class|KismetMathLibrary|DegAcos (Math|Vector|DotProduct (Transformation|GetActorForwardVector) (Math|Vector|Normalize (- (Transformation|GetActorLocation (Variables|Default|GetPlayerReference)) (Transformation|GetActorLocation self))))) 3e+01)
            (CallFunction|Movement)
            (else
              (Components|Movement|StopMovementImmediately (Variables|Character|GetCharacterMovement))
              (CallFunction|StartAttack))))))))

(fn ConstructionScript)