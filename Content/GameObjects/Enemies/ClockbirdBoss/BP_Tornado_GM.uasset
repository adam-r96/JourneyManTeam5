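; BP_Tornado_GM is a tornado hazard for the Clockbird boss that damages the player on overlap with its hitbox.
; BeginPlay applies its scale after a short delay, randomizes curve direction and strength, and starts a despawn timer.
; Tick moves it along local forward, straight for the first second, then optionally yaws it each frame for a curved path.
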(event OnComponentBeginOverlap(TornadoHitbox)
  (params (OverlappedComponent :type Primitive%20Component%20Object%20Reference) (OtherActor :type Actor%20Object%20Reference) (OtherComp :type Primitive%20Component%20Object%20Reference) (OtherBodyIndex :type Integer) (bFromSweep :type Boolean) (SweepResult :type Hit%20Result%20Structure%20%28by%20ref%29))
  ;[0.15 0.15 0.15 0.5] Damage Player if overlapped
  (bind _asbp_third_person_character_ajr (Utilities|Casting|CastToBP_ThirdPersonCharacter_AJR OtherActor))
  (Default|DamagePlayer _asbp_third_person_character_ajr))

(event Custom|Despawn
  ;[0.15 0.15 0.15 0.5] Despawn Tornado
  (Actor|DestroyActor))

(event EventBeginPlay
  ;[0.15 0.15 0.15 0.5] Set the Scale, Curve Duration and Strength of Tornado, and start despawn timer
  (Utilities|FlowControl|Delay 0.1)
  (Transformation|SetActorScale3D (Math|Vector|MakeVector (Variables|Default|GetTornadoScale) (Variables|Default|GetTornadoScale) (Variables|Default|GetTornadoScale)))
  (Variables|Default|SetCurveDirection (Math|Random|RandomFloatinRange -1.0 1.0))
  (Variables|Default|SetCurveStrength (Math|Random|RandomFloatinRange 1e+01 (Variables|Default|GetMaxCurveStrength)))
  (Utilities|Time|SetTimerbyFunctionName 0 "Despawn" (Variables|Default|GetDespawnTimer)))

(event EventTick
  (params (DeltaSeconds :type Float%20%28single-precision%29))
  (if (Variables|Default|GetIsMovingForward)
    (bind _output_get (Variables|Default|SetForwardTimer (+ (Variables|Default|GetForwardTimer) DeltaSeconds)))
    (if (>= _output_get 1.0)
      (Variables|Default|SetIsMovingForward false)
      (else
        (Transformation|AddActorLocalOffset (Math|Vector|MakeVector (* (Variables|Default|GetTornadoSpeed) DeltaSeconds) 0.0 0.0) false false)))
    (else
      (if (Variables|Default|GetShouldCurve)
        (Transformation|AddActorLocalRotation (Math|Rotator|MakeRotator 0.0 0.0 (* (* (Variables|Default|GetCurveDirection) (Variables|Default|GetCurveStrength)) DeltaSeconds)) false false))
      (Transformation|AddActorLocalOffset (Math|Vector|MakeVector (* (Variables|Default|GetTornadoSpeed) DeltaSeconds) 0.0 0.0) false false))))

(fn ConstructionScript)