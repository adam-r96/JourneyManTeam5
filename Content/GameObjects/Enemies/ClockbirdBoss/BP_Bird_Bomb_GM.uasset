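; Bomb actor for the Clockbird boss that damages the player character when it explodes.
; Tick treats near-zero vertical velocity as landing, then runs a three-second fuse that lerps a dynamic material from yellow to red.
; Explode fires once, spawning a Niagara effect, briefly toggling ExplosionRadius query collision, damaging overlapping players and destroying the actor.
; ExplosionRadius begin-overlap events also damage the player directly.
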(event OnComponentBeginOverlap(ExplosionRadius)
  (params (OverlappedComponent :type Primitive%20Component%20Object%20Reference) (OtherActor :type Actor%20Object%20Reference) (OtherComp :type Primitive%20Component%20Object%20Reference) (OtherBodyIndex :type Integer) (bFromSweep :type Boolean) (SweepResult :type Hit%20Result%20Structure%20%28by%20ref%29))
  (bind _asbp_third_person_character_ajr (Utilities|Casting|CastToBP_ThirdPersonCharacter_AJR OtherActor))
  (Default|DamagePlayer _asbp_third_person_character_ajr))

(event Custom|Explode
  (bind _explosionradius (Variables|Default|GetExplosionRadius))
  (if (not (Variables|Default|GetHasExploded))
    (Variables|Default|SetHasExploded true)
    (Niagara|SpawnSystematLocation "/Game/GameFiles/Models/Enemies/BirdBoss/BirdBomb/NS_Explosion_GM.NS_Explosion_GM" (Transformation|GetActorLocation))
    (Collision|SetCollisionEnabled _explosionradius "QueryOnly")
    (Collision|SetCollisionEnabled _explosionradius "NoCollision")
    (for _array_element (Collision|GetOverlappingActors _explosionradius 0 :!class /Script/Engine.PrimitiveComponent)
      (bind _asbp_third_person_character_ajr (Utilities|Casting|CastToBP_ThirdPersonCharacter_AJR _array_element))
      (Default|DamagePlayer _asbp_third_person_character_ajr))
    (Actor|DestroyActor)))

(event EventBeginPlay
  (bind _returnvalue (Rendering|Material|CreateDynamicMaterialInstance (Variables|Default|GetSM_Bomb) 0 "/Game/GameFiles/Materials/Special/M_Bomb_GM.M_Bomb_GM" "None" :!class /Script/Engine.PrimitiveComponent))
  (Variables|Default|SetBombMaterial _returnvalue)
  (Transformation|AddActorWorldOffset "0, 0, 0")
  (Variables|Default|SetGravityScale (Variables|Default|GetGravityScale)))

(event EventTick
  (params (DeltaSeconds :type Float%20%28single-precision%29))
  (if (Variables|Default|GetHasLanded)
    (bind _output_get (Variables|Default|SetDetonationTimer (+ (Variables|Default|GetDetonationTimer) DeltaSeconds)))
    (if (>= _output_get 3.0)
      (CallFunction|Explode)
      (else
        (Rendering|Material|SetVectorParameterValue (Variables|Default|GetBombMaterial) "BombColour" (Math|Color|Lerp(LinearColor) "(R=1.000000,G=1.000000,B=0.000000,A=1.000000)" "(R=1.000000,G=0.000000,B=0.000000,A=1.000000)" (/ (Variables|Default|GetDetonationTimer) 3.0)) :!class /Script/Engine.MaterialInstanceDynamic)))
    (elif (< (Math|Float|Absolute(Float) (.z (Transformation|GetVelocity self))) 1e+01)
      (Variables|Default|SetHasLanded true))))

(fn ConstructionScript)