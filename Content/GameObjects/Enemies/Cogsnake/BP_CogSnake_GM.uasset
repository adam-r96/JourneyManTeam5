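; BP_CogSnake_GM is the head of a Cogsnake enemy that patrols a looping list of waypoints, trailed by a chain of body nodes.
; On BeginPlay it spawns scaled BP_CogSnakeNode_GM segments in a line along its negative right vector.
; Each Tick it interpolates toward the current waypoint, advancing when close.
; Each node eases toward the one ahead, the first following the head, and turns with a yaw offset for sideways-oriented segments.
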(event EventBeginPlay
  (for _index (range 0 (- (Variables|Default|GetNodeCount) 1))
    (bind _returnvalue (Game|SpawnActorfromClass "/Game/GameObjects/Enemies/Cogsnake/BP_CogSnakeNode_GM.BP_CogSnakeNode_GM_C" (Math|Transform|MakeTransform (+ (Transformation|GetActorLocation) (* (Math|Vector|NegateVector (* _index (Variables|Default|GetNodeSpacing))) (Transformation|GetActorRightVector))) (Transformation|GetActorRotation) "1.000000,1.000000,1.000000") "Undefined" "MultiplyWithRoot" self 0))
    (Transformation|SetActorScale3D _returnvalue (Math|Conversions|ToVector(Float) (Variables|Default|GetNodeScale)))
    (Utilities|Array|Add (Variables|Default|GetSpawnedNodes) _returnvalue)))

(event EventTick
  (params (DeltaSeconds :type Float%20%28single-precision%29))
  (Transformation|SetActorLocation (Math|Interpolation|VInterpTo (Transformation|GetActorLocation) (Transformation|GetActorLocation (Utilities|Array|Get(acopy) (Variables|Default|GetWaypoints) (Variables|Default|GetCurrentWaypointIndex))) DeltaSeconds (Variables|Default|GetMovementSpeed)) false false)
  (if (<= (Math|Vector|Distance(Vector) (Transformation|GetActorLocation) (Transformation|GetActorLocation (Utilities|Array|Get(acopy) (Variables|Default|GetWaypoints) (Variables|Default|GetCurrentWaypointIndex)))) 5e+01)
    (Variables|Default|SetCurrentWaypointIndex (Math|Integer|%(Integer) (+ (Variables|Default|GetCurrentWaypointIndex) 1) (Utilities|Array|Length (Variables|Default|GetWaypoints)))))
  (for (_array_element _array_index) (Variables|Default|GetSpawnedNodes)
    (Utilities|IsValid _array_element
      (:Is%20Valid
        (if true
          (Transformation|SetActorLocation _array_element (Math|Interpolation|VInterpTo (Transformation|GetActorLocation _array_element) (select (== _array_index 0) (Transformation|GetActorLocation) (Transformation|GetActorLocation (Utilities|Array|Get(acopy) (Variables|Default|GetSpawnedNodes) (Math|Integer|Max(Integer) (- _array_index 1))))) DeltaSeconds (Variables|Default|GetMovementSpeed)) false false)
          (Transformation|SetActorRotation _array_element (Math|Interpolation|RInterpTo (Transformation|GetActorRotation _array_element) (Math|Rotator|MakeRotator (.Roll (Math|Rotator|BreakRotator (Math|Rotator|FindLookatRotation (Transformation|GetActorLocation _array_element) (select (== _array_index 0) (Transformation|GetActorLocation (Utilities|Array|Get(acopy) (Variables|Default|GetWaypoints) (Variables|Default|GetCurrentWaypointIndex))) (Transformation|GetActorLocation (Utilities|Array|Get(acopy) (Variables|Default|GetSpawnedNodes) (Math|Integer|Max(Integer) (- _array_index 1)))))))) (.Pitch (Math|Rotator|BreakRotator (Math|Rotator|FindLookatRotation (Transformation|GetActorLocation _array_element) (select (== _array_index 0) (Transformation|GetActorLocation (Utilities|Array|Get(acopy) (Variables|Default|GetWaypoints) (Variables|Default|GetCurrentWaypointIndex))) (Transformation|GetActorLocation (Utilities|Array|Get(acopy) (Variables|Default|GetSpawnedNodes) (Math|Integer|Max(Integer) (- _array_index 1)))))))) (- (.Yaw (Math|Rotator|BreakRotator (Math|Rotator|FindLookatRotation (Transformation|GetActorLocation _array_element) (select (== _array_index 0) (Transformation|GetActorLocation (Utilities|Array|Get(acopy) (Variables|Default|GetWaypoints) (Variables|Default|GetCurrentWaypointIndex))) (Transformation|GetActorLocation (Utilities|Array|Get(acopy) (Variables|Default|GetSpawnedNodes) (Math|Integer|Max(Integer) (- _array_index 1)))))))) 9e+01)) DeltaSeconds 3.0)))))))

(fn ConstructionScript)