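; BP_VFX_HoverBoots is the visual effect actor for the hover boots ability, a Niagara beam reaching down to the floor.
; Each tick it line traces straight down against world static and dynamic objects and feeds the hit point, or the trace end on a miss, to the beam's end parameter.
; Stop deactivates the Niagara system without a reset, and the actor destroys itself once the system finishes.
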(event OnSystemFinished(Niagara)
  (params (PSystem :type Niagara%20Component%20Object%20Reference))
  (Actor|DestroyActor))

(event Custom|Stop
  (Components|Activation|SetActive (Variables|Default|GetNiagara) false false))

(event EventTick
  (params (DeltaSeconds :type Float%20%28single-precision%29))
  (bind _returnvalue (Transformation|GetActorLocation))
  ;[0.15 0.15 0.15 0.5] Linetrace for a floor to assign the bottom of the laser to
  (bind _outhit (Collision|LineTraceForObjects _returnvalue (- _returnvalue "0.000000,0.000000,10000.000000") (Utilities|Array|MakeArray "ObjectTypeQuery1" "ObjectTypeQuery2") false 0 "None"))
  ;[0.15 0.15 0.15 0.5] Set the target beam end location to the hit location if one was found, if not set it to the trace's end location.
  (Effects|Components|ParticleSystem|SetVectorParameter (Variables|Default|GetNiagara) "Beam End" (Math|Vector|SelectVector (.Location (Collision|BreakHitResult _outhit)) (.TraceEnd (Collision|BreakHitResult _outhit)) (.bBlockingHit (Collision|BreakHitResult _outhit)))))

(fn ConstructionScript)