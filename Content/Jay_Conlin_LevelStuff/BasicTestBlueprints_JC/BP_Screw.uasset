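; BP_Screw is a one-shot interactable screw that animates when the player walks into its box, flagging that a door can open.
; Unless Stop is set, the overlap plays the ScrewDown timeline, whose vector track drives the mesh's Z offset from the Scene component and its yaw.
; The first timeline update also plays a 2D sound, sets Done and destroys the Niagara and point light components.
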(event OnComponentBeginOverlap(Box)
  (params (OverlappedComponent :type Primitive%20Component%20Object%20Reference) (OtherActor :type Actor%20Object%20Reference) (OtherComp :type Primitive%20Component%20Object%20Reference) (OtherBodyIndex :type Integer) (bFromSweep :type Boolean) (SweepResult :type Hit%20Result%20Structure%20%28by%20ref%29))
  (bind _staticmesh (Variables|Default|GetStaticMesh))
  (bind _scene (Variables|Default|GetScene))
  (bind _relativerotation (Variables|/Script/Engine.SceneComponent|GetRelativeRotation _staticmesh))
  (bind _relativelocation (Variables|/Script/Engine.SceneComponent|GetRelativeLocation _scene))
  (if (== OtherActor (Game|GetPlayerCharacter 0))
    (if (not (Variables|Default|GetStop))
      (Utilities|FlowControl|DoOnce false
        (:Completed
          (Variables|Default|SetStart (.z (Variables|/Script/Engine.SceneComponent|GetRelativeLocation _staticmesh)))
          (bind _screwdown (Timeline|Timeline Play)
            (:Update
              (Transformation|SetRelativeRotation _staticmesh (Math|Rotator|MakeRotator (.roll _relativerotation) (.pitch _relativerotation) (.Y (Math|Vector|BreakVector _screwdown))) false false)
              (Transformation|SetRelativeLocation _staticmesh (Math|Vector|MakeVector (.x _relativelocation) (.y _relativelocation) (+ (.z _relativelocation) (.X (Math|Vector|BreakVector _screwdown)))) false false)
              (Variables|Default|SetCanOpenDoor true)
              (Utilities|FlowControl|DoOnce false
                (:Completed
                  (Audio|PlaySound2D "/Engine/EditorSounds/GamePreview/StartPlayInEditor_Cue.StartPlayInEditor_Cue" 0.6 1.0 0.0 0 0)
                  (Variables|Default|SetDone? true)
                  (Components|DestroyComponent (Variables|Default|GetNiagara)))))))))))

(event EventBeginPlay)

(event Collision|EventActorBeginOverlap
  (params (OtherActor :type Actor%20Object%20Reference)))

(fn ConstructionScript)