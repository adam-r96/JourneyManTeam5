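; BP_Rod_JC is a rod actor that animates the Z scale of a static mesh with a timeline.
; While not stopped, Tick waits a configurable delay and plays the timeline, whose update drives StaticMesh's height and holds StaticMesh1 at full height.
; When Stopped is set, a DoOnce flattens both meshes to zero Z scale and stops the timeline.
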(event EventBeginPlay)

(event Collision|EventActorBeginOverlap
  (params (OtherActor :type Actor%20Object%20Reference)))

(event EventTick
  (params (DeltaSeconds :type Float%20%28single-precision%29))
  (bind _staticmesh (Variables|Default|GetStaticMesh))
  (bind _staticmesh1 (Variables|Default|GetStaticMesh1))
  (if (Variables|Default|GetStopped?)
    (Utilities|FlowControl|DoOnce false
      (:Completed
        (Transformation|SetWorldScale3D _staticmesh (Math|Vector|MakeVector 1.75 1.75 0.0))
        (Transformation|SetWorldScale3D _staticmesh1 (Math|Vector|MakeVector 1.75 1.75 0.0))
        (bind _newtrack_0 (Timeline|Timeline Stop)
          (:Update
            (Transformation|SetWorldScale3D _staticmesh (Math|Vector|MakeVector 1.75 1.75 _newtrack_0))
            (Transformation|SetWorldScale3D _staticmesh1 (Math|Vector|MakeVector 1.75 1.75 1.0))
            (Timeline|Timeline Play)))))
    (else
      (Utilities|FlowControl|Delay (Variables|Default|GetDelayTime))
      (Timeline|Timeline Play))))

(fn ConstructionScript)