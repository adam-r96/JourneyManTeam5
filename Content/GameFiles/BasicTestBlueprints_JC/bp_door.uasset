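; A test door actor that opens once a linked screw reports it can open the door.
; Tick polls the screw's flag when a door is needed and uses a DoOnce to trigger the opening sequence a single time.
; After a short delay, a timeline animates the Scene component's Z scale while keeping X and Y unchanged.
; The same sequence is also reachable through an Open event.
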(event Custom|Open
  (bind _scene (Variables|Default|GetScene))
  (bind _relativescale3d (Variables|/Script/Engine.SceneComponent|GetRelativeScale3D _scene))
  (Utilities|FlowControl|Delay 1.0)
  (bind _oipen (Timeline|Timeline Play)
    (:Update
      (Transformation|SetRelativeScale3D _scene (Math|Vector|MakeVector (.x _relativescale3d) (.y _relativescale3d) _oipen)))))

(event EventBeginPlay)

(event Collision|EventActorBeginOverlap
  (params (OtherActor :type Actor%20Object%20Reference)))

(event EventTick
  (params (DeltaSeconds :type Float%20%28single-precision%29))
  (bind _scene (Variables|Default|GetScene))
  (bind _relativescale3d (Variables|/Script/Engine.SceneComponent|GetRelativeScale3D _scene))
  (if (Variables|Default|GetnEEDSdOOR?)
    (if (Variables|/Game/GameFiles/BasicTestBlueprints_JC/BP_Screw.BP_Screw_C|GetCanOpenDoor (Variables|Default|Getscrew))
      (Utilities|FlowControl|DoOnce false
        (:Completed
          (Utilities|FlowControl|Delay 1.0)
          (bind _oipen (Timeline|Timeline Play)
            (:Update
              (Transformation|SetRelativeScale3D _scene (Math|Vector|MakeVector (.x _relativescale3d) (.y _relativescale3d) _oipen)))))))))

(fn ConstructionScript)